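; BP_Arrow is a laser emitter Actor with colored beam and impact particles, plus a sphere that deals damage to an overlapping first-person character.
; Each tick it line traces along the Arrow component to set the beam's end point and show the impact at blocking hits.
; Beam length grows over time up to MaxDistance and shortens to the hit distance when blocked.
; An unfinished reflection step is left unconnected.
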(event OnComponentBeginOverlap(Sphere)
  (params (OverlappedComponent :type Primitive%20Component%20Object%20Reference) (OtherActor :type Actor%20Object%20Reference) (OtherComp :type Primitive%20Component%20Object%20Reference) (OtherBodyIndex :type Integer) (bFromSweep :type Boolean) (SweepResult :type Hit%20Result%20Structure%20%28by%20ref%29))
  (bind _asbp_first_person_character (Utilities|Casting|CastToBP_FirstPersonCharacter OtherActor))
  (Game|Damage|ApplyDamage _asbp_first_person_character 1e+02 0 0))

(event EventBeginPlay
  (Components|Activation|SetActive (Variables|Default|GetLaser) true false)
  (Effects|Components|ParticleSystem|SetColorParameter (Variables|Default|GetImpact) "Color" "(R=0.152778,G=0.000000,B=0.002153,A=1.000000)"))

(event EventTick
  (params (DeltaSeconds :type Float%20%28single-precision%29))
  (bind _arrow (Variables|Default|GetArrow))
  (bind _returnvalue (Transformation|GetWorldLocation _arrow))
  (Utilities|FlowControl|Sequence
    (:then_0
      (bind _output_get (Variables|Default|SetTraceEnd (+ _returnvalue (* (Math|Vector|GetForwardVector _arrow) (Variables|Default|GetDistance)))))
      (bind _outhit (Collision|LineTraceByChannel _returnvalue _output_get "TraceTypeQuery2" false 0 "ForOneFrame"))
      (bind _output_get_2 (Variables|Default|SetBlocking%20Hit (.bblockinghit _outhit)))
      (bind _output_get_3 (Variables|Default|SetOut%20Hit%20Location (.location _outhit)))
      (Effects|Components|ParticleSystem|SetVectorParameter (Variables|Default|GetLaser) "Laser End Point" (select _output_get_2 _output_get_3 (Variables|Default|GetTraceEnd)))
      (Rendering|SetVisibility (Variables|Default|GetImpact) _output_get_2 false)
      (Transformation|SetWorldLocation (Variables|Default|GetImpact) (Variables|Default|GetOut%20Hit%20Location) false false)
      (if (Variables|Default|GetBlocking%20Hit)
        (Variables|Default|SetDistance (Math|Vector|VectorLength (- (Variables|Default|GetOut%20Hit%20Location) (Transformation|GetActorLocation))))))
    (:then_1
      (if (< (Variables|Default|GetDistance) (Variables|Default|GetMaxDistance))
        (Variables|Default|SetDistance (+ (Variables|Default|GetDistance) (* DeltaSeconds (Variables|Default|GetIncDistance))))))))

(fn ConstructionScript)