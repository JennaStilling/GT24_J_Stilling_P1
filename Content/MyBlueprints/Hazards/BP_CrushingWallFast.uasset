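; BP_CrushingWallFast is a hazard whose wall repeatedly slides along its local Z axis and damages a player caught by it.
; After an initial delay, the Movement timeline drives a swept relative move of Wall, then replays after a restart delay.
; A Box overlap flags the first-person character's presence, and a blocking sweep hit while flagged applies damage to player 0's pawn.
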(event OnComponentBeginOverlap(Box)
  (params (OverlappedComponent :type Primitive%20Component%20Object%20Reference) (OtherActor :type Actor%20Object%20Reference) (OtherComp :type Primitive%20Component%20Object%20Reference) (OtherBodyIndex :type Integer) (bFromSweep :type Boolean) (SweepResult :type Hit%20Result%20Structure%20%28by%20ref%29))
  (Utilities|Casting|CastToBP_FirstPersonCharacter OtherActor)
  (Variables|Default|SetisOverlapping true)
  (Development|PrintString "Hello"))

(event OnComponentEndOverlap(Box)
  (params (OverlappedComponent :type Primitive%20Component%20Object%20Reference) (OtherActor :type Actor%20Object%20Reference) (OtherComp :type Primitive%20Component%20Object%20Reference) (OtherBodyIndex :type Integer))
  (Utilities|Casting|CastToBP_FirstPersonCharacter OtherActor)
  (Variables|Default|SetisOverlapping false))

(event Custom|Smash
  (bind _motion (Timeline|Movement PlayFromStart)
    (:Update
      (bind _sweephitresult (Transformation|SetRelativeLocation (Variables|Default|GetWall) (Math|Vector|Lerp(Vector) "0.000000,0.000000,500.000000" "0, 0, 0" _motion) true false))
      (if (and (.bblockinghit _sweephitresult) (Variables|Default|GetisOverlapping))
        (bind _asbp_first_person_character (Utilities|Casting|CastToBP_FirstPersonCharacter (Game|Player|GetPlayerPawn 0)))
        (Game|Damage|ApplyDamage _asbp_first_person_character 1e+02 0 0)))
    (:Finished
      (Utilities|FlowControl|Delay (Variables|Default|GetRestartDelay))
      (CallFunction|Smash))))

(event EventBeginPlay
  (Utilities|FlowControl|Delay (Variables|Default|GetDelay))
  (CallFunction|Smash))

(fn ConstructionScript)