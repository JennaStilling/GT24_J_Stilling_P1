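; Swinging axe hazard that rotates between +80 and -80 degrees of pitch and deals 100 damage to the first-person character.
; After a start delay, the Movement timeline lerps the Scene component's relative rotation and calls Swing again on finish to loop.
; Speed values other than 3.0 set the play rate to 1/Speed, so higher values swing slower.
; Damage triggers when the character begins overlapping Sphere1.
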(event OnComponentBeginOverlap(Sphere1)
  (params (OverlappedComponent :type Primitive%20Component%20Object%20Reference) (OtherActor :type Actor%20Object%20Reference) (OtherComp :type Primitive%20Component%20Object%20Reference) (OtherBodyIndex :type Integer) (bFromSweep :type Boolean) (SweepResult :type Hit%20Result%20Structure%20%28by%20ref%29))
  (bind _asbp_first_person_character (Utilities|Casting|CastToBP_FirstPersonCharacter OtherActor))
  (Game|Damage|ApplyDamage _asbp_first_person_character 1e+02 0 0))

(event Custom|Swing
  (bind _movement (Variables|Default|GetMovement))
  (bind _returnvalue (Components|Timeline|GetTimelineLength _movement))
  (if (== (Variables|Default|GetSpeed) 3.0)
    (bind _motion (Timeline|Movement PlayFromStart)
      (:Update
        (Transformation|SetRelativeRotation (Variables|Default|GetScene) (Math|Rotator|Lerp(Rotator) "80.000000,0.000000,0.000000" "-80.000000,0.000000,0.000000" _motion) false false))
      (:Finished
        (CallFunction|Swing)))
    (else
      (Components|Timeline|SetPlayRate _movement (/ _returnvalue (* _returnvalue (Variables|Default|GetSpeed))))
      (Timeline|Movement PlayFromStart))))

(event EventBeginPlay
  (Utilities|FlowControl|Delay (Variables|Default|GetDelay))
  (CallFunction|Swing))

(fn ConstructionScript)