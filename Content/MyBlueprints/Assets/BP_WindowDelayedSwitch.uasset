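; BP_WindowDelayedSwitch is a window that opens once enough switches are active at the same time.
; SwitchActivated and SwitchDeactivated events adjust an active count and compare it to SwitchesNeeded.
; When the threshold is met, a timeline plays to raise the Window component along Z; otherwise it reverses to lower it.
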(event Custom|SwitchDeactivated
  (Math|Integer|DecrementInt (Variables|Default|GetSwitchesActive)
    (:%20%20
      (if (>= (Variables|Default|GetSwitchesActive) (Variables|Default|GetSwitchesNeeded))
        (bind _openwindow (Timeline|OpenWindow%20Timeline Play)
          (:Update
            (Transformation|SetRelativeLocation (Variables|Default|GetWindow) (Math|Vector|MakeVector 0.0 0.0 (* _openwindow 105.0)) false false)))
        (else
          (Timeline|OpenWindow%20Timeline Reverse))))))

(event Custom|SwitchActivated
  (Math|Integer|IncrementInt (Variables|Default|GetSwitchesActive)
    (:%20%20
      (if (>= (Variables|Default|GetSwitchesActive) (Variables|Default|GetSwitchesNeeded))
        (bind _openwindow (Timeline|OpenWindow%20Timeline Play)
          (:Update
            (Transformation|SetRelativeLocation (Variables|Default|GetWindow) (Math|Vector|MakeVector 0.0 0.0 (* _openwindow 105.0)) false false)))
        (else
          (Timeline|OpenWindow%20Timeline Reverse))))))

(fn ConstructionScript)