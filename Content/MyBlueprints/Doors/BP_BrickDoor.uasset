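; BP_BrickDoor is a door that opens once enough switches are active.
; SwitchActivated and SwitchDeactivated adjust an active-switch count and compare it to the required number.
; Meeting the threshold plays a timeline that drives the door's relative Z position, and falling short reverses the same timeline to close it.
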(event Custom|SwitchDeactivated
  (Math|Integer|DecrementInt (Variables|Default|GetSwitchesActive)
    (:%20%20
      (if (>= (Variables|Default|GetSwitchesActive) (Variables|Default|GetSwitchesNeeded))
        (bind _opendoor (Timeline|OpenDoor%20Timeline Play)
          (:Update
            (Transformation|SetRelativeLocation (Variables|Default|GetDoor) (Math|Vector|MakeVector 0.0 0.0 (* _opendoor 205.0)) false false)))
        (else
          (Timeline|OpenDoor%20Timeline Reverse))))))

(event Custom|SwitchActivated
  (Math|Integer|IncrementInt (Variables|Default|GetSwitchesActive)
    (:%20%20
      (if (>= (Variables|Default|GetSwitchesActive) (Variables|Default|GetSwitchesNeeded))
        (bind _opendoor (Timeline|OpenDoor%20Timeline Play)
          (:Update
            (Transformation|SetRelativeLocation (Variables|Default|GetDoor) (Math|Vector|MakeVector 0.0 0.0 (* _opendoor 205.0)) false false)))
        (else
          (Timeline|OpenDoor%20Timeline Reverse))))))

(fn ConstructionScript)