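; BP_CobblestonePressurePad is a pressure pad that activates a linked door when an actor with the required tag overlaps it.
; On the first valid overlap it latches as pressed, calls SwitchActivated on the door, swaps the switch material and moves the switch vertically with a timeline.
; End overlap does nothing, so the pad stays pressed; the release logic that checks remaining tagged actors is present but unconnected.
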(event Collision|EventActorBeginOverlap
  (params (OtherActor :type Actor%20Object%20Reference))
  (if (Actor|ActorHasTag OtherActor (Variables|Default|GetNeededTag))
    (if (not (Variables|Default|GetisPressed))
      (Variables|Default|SetisPressed true)
      (Default|SwitchActivated (Variables|Default|GetDoorToActivate))
      (Rendering|Material|SetMaterial (Variables|Default|GetSwitch) 0 "/Game/MyMaterials/M_SwitchOn.M_SwitchOn")
      (bind _switchposition (Timeline|SwitchActivate Play)
        (:Update
          (Transformation|SetRelativeLocation (Variables|Default|GetSwitch) (Math|Vector|MakeVector 0.0 0.0 _switchposition) false false))))))

(event Collision|EventActorEndOverlap
  (params (OtherActor :type Actor%20Object%20Reference)))

(fn ConstructionScript)