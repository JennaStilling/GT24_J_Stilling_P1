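; BP_DoorPressureSwitch is a pressure pad that activates its linked door while weighted by an actor carrying the required tag.
; A matching overlap notifies the door, swaps the switch material and plays a timeline that moves the switch on Z.
; On end overlap it rechecks all overlapping actors, releasing only when none has the tag, then deactivates the door, restores the off material and reverses the motion.
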(event Collision|EventActorBeginOverlap
  (params (OtherActor :type Actor%20Object%20Reference))
  (if (Actor|ActorHasTag OtherActor (Variables|Default|GetNeededTag))
    (if (not (Variables|Default|GetisPressed))
      (Variables|Default|SetisPressed true)
      (Default|SwitchActivated (Variables|Default|GetDoorToActivate))
      (Rendering|Material|SetMaterial (Variables|Default|GetSwitch) 0 "/Game/MyMaterials/M_SwitchOn.M_SwitchOn")
      (bind _switchposition (Timeline|SwitchActivate Play)
        (:Update
          (Transformation|SetRelativeLocation (Variables|Default|GetSwitch) (Math|Vector|MakeVector 0.0 0.0 _switchposition) false false))))))

(event Collision|EventActorEndOverlap
  (params (OtherActor :type Actor%20Object%20Reference))
  (Variables|Default|SetisWeighted false)
  (for _array_element (Collision|GetOverlappingActors 0 :!class /Script/Engine.Actor)
    (if (Actor|ActorHasTag _array_element (Variables|Default|GetNeededTag))
      (Variables|Default|SetisWeighted true)))
  (if (not (Variables|Default|GetisWeighted))
    (if (not (not (Variables|Default|GetisPressed)))
      (Variables|Default|SetisPressed false)
      (Default|SwitchDeactivated (Variables|Default|GetDoorToActivate))
      (Rendering|Material|SetMaterial (Variables|Default|GetSwitch) 0 "/Game/MyMaterials/M_SwitchOff.M_SwitchOff")
      (bind _switchposition (Timeline|Timeline Reverse)
        (:Update
          (Transformation|SetRelativeLocation (Variables|Default|GetSwitch) (Math|Vector|MakeVector 0.0 0.0 _switchposition) false false))))))

(fn ConstructionScript)