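; Level switch that, going by its name, is meant to be shot, and that activates a linked door.
; Any overlap on its Box latches it on once: it calls SwitchActivated on DoorToActivate, swaps to the on material and moves the switch on Z via a timeline.
; The tag-based release logic is unconnected, so the switch never deactivates; a debug "Hello" prints on each Box overlap.
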(event OnComponentBeginOverlap(Box)
  (params (OverlappedComponent :type Primitive%20Component%20Object%20Reference) (OtherActor :type Actor%20Object%20Reference) (OtherComp :type Primitive%20Component%20Object%20Reference) (OtherBodyIndex :type Integer) (bFromSweep :type Boolean) (SweepResult :type Hit%20Result%20Structure%20%28by%20ref%29))
  (Development|PrintString "Hello")
  (if true
    (if (not (Variables|Default|GetisPressed))
      (Variables|Default|SetisPressed true)
      (Default|SwitchActivated (Variables|Default|GetDoorToActivate))
      (Rendering|Material|SetMaterial (Variables|Default|GetSwitch) 0 "/Game/MyMaterials/M_SwitchOn.M_SwitchOn")
      (bind _switchposition (Timeline|SwitchActivate Play)
        (:Update
          (Transformation|SetRelativeLocation (Variables|Default|GetSwitch) (Math|Vector|MakeVector 0.0 0.0 _switchposition) false false))))))

(event Collision|EventActorBeginOverlap
  (params (OtherActor :type Actor%20Object%20Reference)))

(event Collision|EventActorEndOverlap
  (params (OtherActor :type Actor%20Object%20Reference)))

(fn ConstructionScript)