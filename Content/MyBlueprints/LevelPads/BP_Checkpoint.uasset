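; BP_Checkpoint is a level pad that sets the player's respawn point when BP_FirstPersonCharacter overlaps its Box trigger.
; On overlap it writes its own actor transform into RespawnTransform on BP_FirstPersonGameMode.
; It then prints that transform as a debug string and adds a new WG_Checkpoint widget to the viewport.
; Nothing guards against repeat triggers, so each overlap saves again and creates another widget.
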(event OnComponentBeginOverlap(Box)
  (params (OverlappedComponent :type Primitive%20Component%20Object%20Reference) (OtherActor :type Actor%20Object%20Reference) (OtherComp :type Primitive%20Component%20Object%20Reference) (OtherBodyIndex :type Integer) (bFromSweep :type Boolean) (SweepResult :type Hit%20Result%20Structure%20%28by%20ref%29))
  (Utilities|Casting|CastToBP_FirstPersonCharacter OtherActor)
  (bind _asbp_first_person_game_mode (Utilities|Casting|CastToBP_FirstPersonGameMode (Game|GetGameMode)))
  (bind _output_get (Variables|/Game/FirstPerson/Blueprints/BP_FirstPersonGameMode.BP_FirstPersonGameMode_C|SetRespawn%20Transform _asbp_first_person_game_mode (Transformation|GetActorTransform)))
  (bind _output_get_2 (Variables|Default|SetLocationString "Checkpoint At: "))
  (Development|PrintString (Utilities|String|Append _output_get_2 (Utilities|String|ToString(Transform) _output_get)))
  (bind _returnvalue (UserInterface|CreateWidget "/Game/MyWidget/WG_Checkpoint.WG_Checkpoint_C"))
  (UserInterface|Viewport|AddtoViewport _returnvalue 0))

(fn ConstructionScript)