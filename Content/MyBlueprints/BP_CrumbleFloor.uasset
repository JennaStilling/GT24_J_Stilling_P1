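; BP_CrumbleFloor is a floor actor, apparently meant to crumble under heavy actors.
; On overlap with an actor tagged "Heavy", it prints a debug string, waits briefly, then deactivates its DefaultSceneRoot; no destruction or fracture call runs.
; Unconnected leftovers include a first-person character cast, DestroyActor and an FS_MasterField spawn at the Box transform, suggesting an unfinished Chaos field-based break.
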(event EventBeginPlay)

(event EventTick
  (params (DeltaSeconds :type Float%20%28single-precision%29)))

(event Collision|EventActorBeginOverlap
  (params (OtherActor :type Actor%20Object%20Reference))
  (if (Actor|ActorHasTag OtherActor "Heavy")
    (Development|PrintString "fsfsd")
    (Utilities|FlowControl|Delay 0.2)
    (Components|Activation|Deactivate (Variables|Default|GetDefaultSceneRoot))))

(fn ConstructionScript)