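; Moving platform that slides its static mesh along the spline of a referenced SplineToUse.
; Each tick it advances a distance by Speed and delta time, then sets the mesh's relative location from the spline's local-space point, keeping its scale.
; BIsLooped flips every tick, so the check that resets distance to zero past the spline's end runs only on alternate frames.
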(event EventBeginPlay)

(event EventTick
  (params (DeltaSeconds :type Float%20%28single-precision%29))
  (Variables|Default|SetDistance (+ (* DeltaSeconds (Variables|Default|GetSpeed)) (Variables|Default|GetDistance)))
  (Transformation|SetRelativeTransform (Variables|Default|GetStaticMesh) (Math|Transform|MakeTransform (.location (Spline|GetTransformatDistanceAlongSpline (Variables|/Game/MyBlueprints/MovingPlatforms/BP_SplinePath.BP_SplinePath_C|GetSpline (Variables|Default|GetSplineToUse)) (Variables|Default|GetDistance) "Local" false)) "0, 0, 0" (Variables|/Script/Engine.SceneComponent|GetRelativeScale3D (Variables|Default|GetStaticMesh))) false false)
  (bind _output_get (Variables|Default|Setb_IsLooped (not (Variables|Default|Getb_IsLooped))))
  (if _output_get
    (if (> (Variables|Default|GetDistance) (Spline|GetSplineLength (Variables|/Game/MyBlueprints/MovingPlatforms/BP_SplinePath.BP_SplinePath_C|GetSpline (Variables|Default|GetSplineToUse))))
      (Variables|Default|SetDistance 0.0))))

(fn ConstructionScript)